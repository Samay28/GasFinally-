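; BP_NPC is a Gameplay Ability System NPC that fights back when damaged and grants experience on death.
; BeginPlay sets up a health bar widget fed by the health attribute set and binds that set's damage and out-of-health delegates.
; Damage turns it toward the instigator, triggers its attack ability, and fires blink and scrolling-damage gameplay cues.
; On death it applies GE_DropExp to the killer at its own ExpLevel, activates the death ability and expires shortly after.
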(event `self.ReceiveBeginPlay`
  (`|ExecutionSequence`
    (:`then_0`
      (bind _returnvalue (`|CreateWidget` "/Game/Widget/WBP_HealthBar.WBP_HealthBar_C"))
      (bind _output_get (set `self.HPBar` _returnvalue))
      (`WidgetComponent.SetWidget` (`self.Widget`) _output_get))
    (:`then_1`
      (bind _returnvalue_2 (`AbilitySystemComponent.GetAttributeSet` (`self.AbilitySystemComponent`) "/Script/GasFinally.HealthAttributeSet"))
      (`/Game/Widget/WBP_HealthBar.SetHealthAttributeSet` _output_get _returnvalue_2))
    (:`then_2`
      ; Checking if health drops using the delegate binded in c++
      (add `HealthAttributeSet.OnOutOfHealth` _returnvalue_2 (delegate `OnOutOfHealthBP`))
      ; Making NPC attack back!
      (add `HealthAttributeSet.OnDamageApplied` _returnvalue_2 (delegate `OnDamageApplyBP`)))))

(event `OnOutOfHealthBP`
  (params (InInstigator :type "Actor Object Reference"))
  ; Checking if health drops using the delegate binded in c++
  (bind _returnvalue (`AbilitySystemComponent.GetAttributeSet` (`self.AbilitySystemComponent`) "/Script/GasFinally.ExpAttributeSet"))
  (bind _explevel_basevalue (break `GameplayAttributeData` (`ExpAttributeSet.ExpLevel` _returnvalue)))
  (`AbilitySystemComponent.BP_ApplyGameplayEffectToTarget` :`self` (`self.AbilitySystemComponent`) :`GameplayEffectClass` "/Game/GASstuff/GameplayEffects/GE_DropExp.GE_DropExp_C" :`Target` (`AbilitySystemBlueprintLibrary.GetAbilitySystemComponent` InInstigator) :`Level` _explevel_basevalue)
  (`AbilitySystemComponent.TryActivateAbilitiesByTag` (`self.AbilitySystemComponent`) (`BlueprintGameplayTagLibrary.MakeGameplayTagContainerFromTag` (struct :`TagName` "Character.Ability.Death")) true)
  (`self.SetLifeSpan` 2.5))

(event `OnDamageApplyBP`
  (params (InInstigator :type "Actor Object Reference") (AppliedDamage :type "Float (single-precision)"))
  (bind _returnvalue (`AbilitySystemBlueprintLibrary.MakeGameplayCueParameters` 0.0 AppliedDamage))
  ; Making NPC attack back!
  (`|ExecutionSequence`
    (:`then_0`
      (`self.K2_SetActorRotation` (`KismetMathLibrary.MakeRotFromX` (- (`self.K2_GetActorLocation` InInstigator) (`self.K2_GetActorLocation`))))
      (`AbilitySystemComponent.TryActivateAbilitiesByTag` (`self.AbilitySystemComponent`) (`BlueprintGameplayTagLibrary.MakeLiteralGameplayTagContainer` (struct :`GameplayTags` (struct :`(TagName` "Character.Ability.Attack")))) true))
    (:`then_1`
      (if (> AppliedDamage 0.0)
        (`GameplayCueFunctionLibrary.ExecuteGameplayCueOnActor` self (struct :`TagName` "GameplayCue.Material.BlinkDamage") _returnvalue)
        (`GameplayCueFunctionLibrary.ExecuteGameplayCueOnActor` self (struct :`TagName` "GameplayCue.Actor.ScrollDamage") _returnvalue)))))

(fn `UserConstructionScript`)