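; GA_Attack is a Gameplay Ability that plays the combo attack montage on the avatar Character.
; On activation it sets the movement mode to None to lock movement, then plays AM_ComboAttack through a PlayMontageAndWait task.
; The ability ends when the montage completes, is interrupted or is cancelled, or at once if the avatar is not a Character.
; Ending the ability restores the Character's movement mode to Walking.
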(event `self.K2_ActivateAbility`
  (bind _ascharacter (cast `Character` (`self.GetAvatarActorFromActorInfo`))
    (:`then`
      (`CharacterMovementComponent.SetMovementMode` (`Character.CharacterMovement` _ascharacter) "MOVE_None" 0)
      (`AbilityTask_PlayMontageAndWait.CreatePlayMontageAndWaitProxy` "Attack Task" "/Game/Variant_Combat/Anims/AM_ComboAttack.AM_ComboAttack"
        (:`OnCompleted`
          _)
        (:`OnInterrupted`
          _)
        (:`OnCancelled`
          _))
      (`self.K2_EndAbility`))
    (:`CastFailed`
      (`self.K2_EndAbility`))))

(event `self.K2_OnEndAbility`
  (params (bWasCancelled :type Boolean))
  (bind _ascharacter (cast `Character` (`self.GetAvatarActorFromActorInfo`)))
  (`CharacterMovementComponent.SetMovementMode` (`Character.CharacterMovement` _ascharacter) "MOVE_Walking" 0))